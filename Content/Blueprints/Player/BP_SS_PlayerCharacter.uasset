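; BP_SS_PlayerCharacter is the player character, which moves and fires BP_SS_PlayerAmmo projectiles.
; On BeginPlay it registers the IMC_SS_Mapping Enhanced Input context with the local player.
; IA_Move feeds movement input along the actor's right and forward vectors, scaled by MovementSpeed.
; IA_Shoot spawns ammo at FirePoint0 through DoFire, rate-limited by a CanFire flag that a FireDelay timer resets.
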(event Custom|SetCanFireTrue
  (Variables|Default|SetCanFire true))

(event Input|EnhancedActionEvents|EnhancedInputActionIA_Move
  (params (ActionValue :type Vector%202D%20Structure) (ElapsedSeconds :type Float%20%28double-precision%29) (TriggeredSeconds :type Float%20%28double-precision%29) (InputAction :type Input%20Action%20Object%20Reference :default "/Game/Blueprints/Input/IA_Move.IA_Move"))
  (Pawn|Input|AddMovementInput (* (Transformation|GetActorRightVector) (Variables|Default|GetMovementSpeed)) (.x ActionValue) false)
  (Pawn|Input|AddMovementInput (* (Transformation|GetActorForwardVector) (Variables|Default|GetMovementSpeed)) (.y ActionValue) false))

(event Input|EnhancedActionEvents|EnhancedInputActionIA_Shoot
  (params (ActionValue :type Boolean) (ElapsedSeconds :type Float%20%28double-precision%29) (TriggeredSeconds :type Float%20%28double-precision%29) (InputAction :type Input%20Action%20Object%20Reference :default "/Game/Blueprints/Input/IA_Shoot.IA_Shoot"))
  (if (Variables|Default|GetCanFire)
    (CallFunction|DoFire)
    (Variables|Default|SetCanFire false)
    (Utilities|Time|SetTimerbyEvent (delegate Custom|SetCanFireTrue) (Variables|Default|GetFireDelay))))

(event EventBeginPlay
  (bind _asplayer_controller (Utilities|Casting|CastToPlayerController (Game|GetPlayerController 0)))
  (Utilities|IsValid (PlayerController|LocalPlayerSubsystems|GetEnhancedInputLocalPlayerSubsystem _asplayer_controller)
    (:Is%20Valid
      (Input|AddMappingContext (PlayerController|LocalPlayerSubsystems|GetEnhancedInputLocalPlayerSubsystem _asplayer_controller) "/Game/Blueprints/Input/IMC_SS_Mapping.IMC_SS_Mapping" 0 "(bIgnoreAllPressedKeysUntilRelease=True,bForceImmediately=False,bNotifyUserSettings=False)"))))

(event Collision|EventActorBeginOverlap
  (params (OtherActor :type Actor%20Object%20Reference)))

(event EventTick
  (params (DeltaSeconds :type Float%20%28single-precision%29)))

(fn ConstructionScript)

(fn DoFire
  (Game|SpawnActorfromClass "/Game/Blueprints/Player/BP_SS_PlayerAmmo.BP_SS_PlayerAmmo_C" (Transformation|GetWorldTransform (Variables|Default|GetFirePoint_0)) "Undefined" "MultiplyWithRoot" 0 6e+02 0))