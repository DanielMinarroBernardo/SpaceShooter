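; BP_SS_EnemyHorizontal is an enemy that moves in a straight horizontal line while firing at regular intervals.
; On BeginPlay it runs the parent logic and stores its right vector as the movement direction.
; Each tick it offsets its location along that vector by speed and delta time, without sweep.
; A timer accumulated in Tick calls Fire, which is not defined here, whenever it exceeds the fire delay.
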(event EventBeginPlay
  (|CallParentFunction)
  (Variables|Default|SetMovementVector (Transformation|GetActorRightVector)))

(event Collision|EventActorBeginOverlap
  (params (OtherActor :type Actor%20Object%20Reference))
  (|CallParentFunction OtherActor) ; This node is disabled and will not be called.\nDrag off pins to build functionality.
)

(event EventTick
  (params (DeltaSeconds :type Float%20%28single-precision%29))
  (CallFunction|MoveHorizontal DeltaSeconds)
  (bind _output_get (Variables|Default|SetShootCurrentTime (+ DeltaSeconds (Variables|Default|GetShootCurrentTime))))
  (if (> _output_get (Variables|Default|GetFireDelay))
    (Variables|Default|SetShootCurrentTime 0.0)
    (CallFunction|Fire)))

(fn ConstructionScript
  (|CallParentFunction))

(fn MoveHorizontal
  (params (DeltaSeconds :type Float%20%28double-precision%29))
  (Transformation|SetActorLocation (+ (* (Variables|Default|GetMovementVector) (* DeltaSeconds (Variables|Default|GetMovementSpeed))) (Transformation|GetActorLocation)) false false))