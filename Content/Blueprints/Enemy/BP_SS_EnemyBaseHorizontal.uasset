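; BP_SS_EnemyBaseHorizontal is an enemy Blueprint that sets a sideways movement direction and fires faster as it bounces between walls.
; It starts along its right vector without calling parent BeginPlay, leaving use of MovementVector to code outside this graph.
; Overlapping a "Wall"-tagged actor flips the direction and shortens FireDelay by a fixed step until MinDelay is reached.
; Other overlaps pass to the parent.
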(event EventBeginPlay
  (Variables|Default|SetMovementVector (Transformation|GetActorRightVector))
  (Variables|Default|SetIsRight? true))

(event Collision|EventActorBeginOverlap
  (params (OtherActor :type Actor%20Object%20Reference))
  (bind _returnvalue (Transformation|GetActorRightVector))
  (if (Actor|ActorHasTag OtherActor "Wall")
    (if (Variables|Default|GetIsRight?)
      (Variables|Default|SetIsRight? false)
      (Variables|Default|SetMovementVector (* _returnvalue -1.0))
      (else
        (Variables|Default|SetIsRight? true)
        (Variables|Default|SetMovementVector _returnvalue)))
    (CallFunction|DecreceFireDelay)
    (else
      (|CallParentFunction OtherActor))))

(event EventTick
  (params (DeltaSeconds :type Float%20%28single-precision%29))
  (|CallParentFunction DeltaSeconds) ; This node is disabled and will not be called.\nDrag off pins to build functionality.
)

(fn ConstructionScript
  (|CallParentFunction))

(fn DecreceFireDelay
  (if (not (<= (Variables|Default|GetFireDelay) (Variables|Default|GetMinDelay)))
    (Variables|Default|SetFireDelay (- (Variables|Default|GetFireDelay) 0.5))))