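; BP_SS_EnemyAmmo is an enemy projectile that flies straight along its forward vector and expires after a set lifespan.
; Tick moves it by teleport-free, non-swept location updates scaled by bullet speed and delta time.
; Overlapping an actor tagged Wall spawns an explosion with sound, then destroys it after a short delay.
; The capsule overlap casts to the player character but takes no further action, so no damage is applied here.
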(event OnComponentBeginOverlap(Capsule)
  (params (OverlappedComponent :type Primitive%20Component%20Object%20Reference) (OtherActor :type Actor%20Object%20Reference) (OtherComp :type Primitive%20Component%20Object%20Reference) (OtherBodyIndex :type Integer) (bFromSweep :type Boolean) (SweepResult :type Hit%20Result%20Structure%20%28by%20ref%29))
  (Utilities|Casting|CastToBP_SS_PlayerCharacter OtherActor))

(event EventBeginPlay
  (Actor|SetLifeSpan (Variables|Default|GetLifeSpan)))

(event Collision|EventActorBeginOverlap
  (params (OtherActor :type Actor%20Object%20Reference))
  (if (Utilities|Array|ContainsItem (Variables|/Script/Engine.Actor|GetTags OtherActor) "Wall")
    (Effects|SpawnEmitteratLocation "/Game/StarterContent/Particles/P_Explosion.P_Explosion" (Transformation|GetActorLocation))
    (Audio|PlaySound2D "/Game/StarterContent/Audio/Explosion01.Explosion01" 1.0 1.0 0.0 0 0)
    (Utilities|FlowControl|Delay 0.2)
    (Actor|DestroyActor)))

(event EventTick
  (params (DeltaSeconds :type Float%20%28single-precision%29))
  (Transformation|SetActorLocation (+ (* (Transformation|GetActorForwardVector) (* DeltaSeconds (Variables|Default|GetBulletSpeed))) (Transformation|GetActorLocation)) false false))

(fn ConstructionScript)