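; Base enemy actor that flies in a straight line, fires projectiles periodically and destroys itself on contact with the player.
; BeginPlay stores the forward vector, and Tick moves the actor along it without sweep while accumulating a timer against FireDelay.
; Each shot spawns BP_SS_EnemyAmmo at FirePoint.
; Overlapping a Player-tagged actor leads to EnemyDestroyed, with short delays before the actor is removed.
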(event Custom|EnemyDestroyed
  (Utilities|FlowControl|Delay 0.2)
  (Actor|DestroyActor))

(event EventBeginPlay
  (Variables|Default|SetMovementVector (Transformation|GetActorForwardVector)))

(event EventTick
  (params (DeltaSeconds :type Float%20%28single-precision%29))
  (CallFunction|Move DeltaSeconds)
  (bind _output_get (Variables|Default|SetShootCurrentTime (+ DeltaSeconds (Variables|Default|GetShootCurrentTime))))
  (if (> _output_get (Variables|Default|GetFireDelay))
    (Variables|Default|SetShootCurrentTime 0.0)
    (CallFunction|Fire)))

(event Collision|EventActorBeginOverlap
  (params (OtherActor :type Actor%20Object%20Reference))
  (if (Actor|ActorHasTag OtherActor "Player")
    (Utilities|FlowControl|Delay 0.2)
    (CallFunction|EnemyDestroyed)))

(fn ConstructionScript)

(fn Move
  (params (DeltaSeconds :type Float%20%28single-precision%29))
  (Transformation|SetActorLocation (+ (* (Variables|Default|GetMovementVector) (* DeltaSeconds (Variables|Default|GetMovementSpeed))) (Transformation|GetActorLocation)) false false))

(fn Fire
  (Game|SpawnActorfromClass "/Game/Blueprints/Enemy/BP_SS_EnemyAmmo.BP_SS_EnemyAmmo_C" (Transformation|GetWorldTransform (Variables|Default|GetFirePoint)) "Undefined" "MultiplyWithRoot" 0 4e+02 0))